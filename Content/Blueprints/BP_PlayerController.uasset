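; BP_PlayerController is the player controller that sets up input and handles simple respawning.
; On BeginPlay it adds the IMC_Default mapping context to the Enhanced Input subsystem.
; On UnPossess, treated as the player's death, it waits one tick, spawns the game mode's default pawn at a found PlayerStart and possesses it.
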(event `self.ReceiveBeginPlay`
  ;[1 1 1] Enhanced Inputを有効にする
  (`EnhancedInputSubsystemInterface.AddMappingContext` (subsystem `EnhancedInputLocalPlayerSubsystem`) "/Game/Inputs/IMC_Default.IMC_Default" 0 (struct)))

(event `self.ReceiveUnPossess`
  (params (UnpossessedPawn :type "Pawn Object Reference"))
  (`KismetSystemLibrary.DelayUntilNextTick`) ; １フレーム待機して...
  ;[1 1 1] 簡易リスポーン処理
  (bind _returnvalue (`|SpawnActorFromClass` (`GameModeBase.DefaultPawnClass` (`GameplayStatics.GetGameMode`)) (`self.GetTransform` (`GameModeBase.K2_FindPlayerStart` (`GameplayStatics.GetGameMode`) self "")) "Undefined" "OverrideRootScale" null null))
  (`self.Possess` self _returnvalue))

(fn `UserConstructionScript`)