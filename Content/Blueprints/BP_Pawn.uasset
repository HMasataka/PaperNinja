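; Player character Blueprint with camera-relative movement, look, sprint and jump through Enhanced Input.
; Jumping from a near standstill waits briefly to act as a charged jump, and sprint toggles max walk speed while held.
; Hits apply damage to the other actor, and a force-kill input damages itself.
; Any damage received triggers a one-time death that disables movement and sets a short life span.
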(event `self.ReceiveTick`
  (params (DeltaSeconds :type "Float (single-precision)")))

(event `self.ReceiveAnyDamage`
  (params (Damage :type "Float (single-precision)") (DamageType :type "DamageType Object Reference") (InstigatedBy :type "Controller Object Reference") (DamageCauser :type "Actor Object Reference"))
  (`/Engine/EditorBlueprintResources/StandardMacros.DoOnce` false ; 死亡処理は一度だけ実行する
    (:`Completed`
      (`KismetSystemLibrary.PrintString` "Died!")
      (`CharacterMovementComponent.DisableMovement` (`self.CharacterMovement`)) ; キャラクターを動けなくする
      (`self.SetLifeSpan` 5.0) ; 5.0秒の寿命をつける
    )))

(event `self.ReceiveHit`
  (params (MyComp :type "PrimitiveComponent Object Reference") (Other :type "Actor Object Reference") (OtherComp :type "PrimitiveComponent Object Reference") (bSelfMoved :type Boolean) (HitLocation :type "Vector Structure") (HitNormal :type "Vector Structure") (NormalImpulse :type "Vector Structure") (Hit :type "HitResult Structure (by ref)"))
  ;[1 1 1] Hit相手にダメージを適用
  (`GameplayStatics.ApplyDamage` Other 1.0 null self))

(event `EnhancedInput|/Game/Inputs/IA_Jump`
  (params (ActionValue :type Boolean) (ElapsedSeconds :type "Float (double-precision)") (TriggeredSeconds :type "Float (double-precision)") (InputAction :type "InputAction Object Reference" :default "/Game/Inputs/IA_Jump.IA_Jump"))
  ;[1 1 1] ジャンプ操作の制御。静止時はタメジャンプをする
  (:`Triggered`
    (if (`self.CanJump`)
      (if (not (>= (`KismetMathLibrary.VSizeXY` (`self.GetVelocity`)) 10.0))
        (`KismetSystemLibrary.Delay` 0.3))
      (`self.Jump`))))

(event `EnhancedInput|/Game/Inputs/IA_Sprint`
  (params (ActionValue :type Boolean) (ElapsedSeconds :type "Float (double-precision)") (TriggeredSeconds :type "Float (double-precision)") (InputAction :type "InputAction Object Reference" :default "/Game/Inputs/IA_Sprint.IA_Sprint"))
  (bind _charactermovement (`self.CharacterMovement`))
  (:`Triggered`
    (set `CharacterMovementComponent.MaxWalkSpeed` 200.0 _charactermovement) ; スプリント時の速度
  )
  (:`Completed`
    (set `CharacterMovementComponent.MaxWalkSpeed` 75.0 _charactermovement) ; 通常歩行時の速度
  ))

(event `EnhancedInput|/Game/Inputs/IA_ForceKill`
  (params (ActionValue :type Boolean) (ElapsedSeconds :type "Float (double-precision)") (TriggeredSeconds :type "Float (double-precision)") (InputAction :type "InputAction Object Reference" :default "/Game/Inputs/IA_ForceKill.IA_ForceKill"))
  ;[1 1 1] フォースキル
  (:`Triggered`
    (`GameplayStatics.ApplyDamage` self 1.0) ; 自分自身にダメージを与える
  ))

(event `EnhancedInput|/Game/Inputs/IA_Look`
  (params (ActionValue :type "Vector2D Structure") (ElapsedSeconds :type "Float (double-precision)") (TriggeredSeconds :type "Float (double-precision)") (InputAction :type "InputAction Object Reference" :default "/Game/Inputs/IA_Look.IA_Look"))
  (bind (_x _y) (`KismetMathLibrary.BreakVector2D` ActionValue))
  ;[1 1 1] カメラ制御
  (:`Triggered`
    (`self.AddControllerYawInput` _x)
    (`self.AddControllerPitchInput` _y)))

(event `EnhancedInput|/Game/Inputs/IA_Move`
  (params (ActionValue :type "Vector2D Structure") (ElapsedSeconds :type "Float (double-precision)") (TriggeredSeconds :type "Float (double-precision)") (InputAction :type "InputAction Object Reference" :default "/Game/Inputs/IA_Move.IA_Move"))
  (bind (_x _y) (`KismetMathLibrary.BreakVector2D` ActionValue))
  ;[1 1 1] 移動
  (:`Triggered`
    (`self.AddMovementInput` (`SceneComponent.GetForwardVector` (`self.Camera`)) _y) ; 前後移動
    (`self.AddMovementInput` (`SceneComponent.GetRightVector` (`self.Camera`)) _x) ; 左右移動
  ))

(fn `UserConstructionScript`)